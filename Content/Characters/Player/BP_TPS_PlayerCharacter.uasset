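; BP_TPS_PlayerCharacter is the third-person player character, adding camera sprint feedback, crouch handling and basic health.
; Sprint start and end events play and reverse a timeline that interpolates the spring arm length between the default cached at BeginPlay and a sprint length.
; Jumping while crouched triggers an uncrouch.
; Incoming damage reduces Health and only prints the remaining value, or "Dead" at zero or below.
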(event `self.ReceiveBeginPlay`
  (set `self.DefaultArmLength` (`SpringArmComponent.TargetArmLength` (`self.SpringArm`))))

(event `OnStartSprint_1`
  (bind (_direction _alpha) (`Timeline|SpringArmSprintTimeline` :!label _label)
    (:`Update`
      (set `SpringArmComponent.TargetArmLength` (`KismetMathLibrary.Lerp` (`self.DefaultArmLength`) (`self.SpringArmLength`) _alpha) (`self.SpringArm`)))))

(event `OnEndSprint_1`
  (goto _label :!via `Reverse`))

(event `self.OnJumped`
  (if (`self.bIsCrouched`)
    (`self.UnCrouch`)))

(event `self.ReceiveAnyDamage`
  (params (Damage :type "Float (single-precision)") (DamageType :type "DamageType Object Reference") (InstigatedBy :type "Controller Object Reference") (DamageCauser :type "Actor Object Reference"))
  (set `self.Health` (- (`self.Health`) Damage))
  (if (<= (`self.Health`) 0.0)
    (`KismetSystemLibrary.PrintString` "Dead" true true (struct :`R` 1.0 :`G` 0.012295 :`A` 1.0))
    (else
      (`KismetSystemLibrary.PrintString` (`KismetStringLibrary.Conv_DoubleToString` (`self.Health`)) true true (struct :`G` 1.0 :`B` 0.04772 :`A` 1.0)))))

(fn `UserConstructionScript`)